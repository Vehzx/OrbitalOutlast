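; BP_Meteor is a physics-driven meteor that bounces off other meteors and damages player characters on contact.
; Tick pushes SMMeteor along CurrentDirection, initially the actor's forward vector, using delta-scaled, mass-independent force.
; Collider overlaps with another meteor call ApplyReflection, which reflects the actor's forward vector (not CurrentDirection) off the impact normal, applies an impulse and updates CurrentDirection.
; Overlapping a BP_Character applies damage and destroys the meteor.
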(event OnComponentBeginOverlap(Collider)
  (params (OverlappedComponent :type Primitive%20Component%20Object%20Reference) (OtherActor :type Actor%20Object%20Reference) (OtherComp :type Primitive%20Component%20Object%20Reference) (OtherBodyIndex :type Integer) (bFromSweep :type Boolean) (SweepResult :type Hit%20Result%20Structure%20%28by%20ref%29))
  (bind _asbp_meteor (Utilities|Casting|CastToBP_Meteor OtherActor)
    (:then
      (CallFunction|ApplyReflection _asbp_meteor (.impactnormal SweepResult)))
    (:CastFailed
      (bind _asbp_character (Utilities|Casting|CastToBP_Character OtherActor))
      (Game|Damage|ApplyDamage _asbp_character 1e+01 0 self)
      (Actor|DestroyActor))))

(event EventBeginPlay
  (Variables|Default|SetCurrentDirection (Transformation|GetActorForwardVector)))

(event Collision|EventActorBeginOverlap
  (params (OtherActor :type Actor%20Object%20Reference)))

(event EventTick
  (params (DeltaSeconds :type Float%20%28single-precision%29))
  (Physics|AddForce (Variables|Default|GetSM_Meteor) (* (Variables|Default|GetCurrentDirection) 1e+04 DeltaSeconds) "None" true))

(fn ConstructionScript)

(fn ApplyReflection
  (params (HitMeteor :type BP%20Meteor%20Object%20Reference) (SurfaceNormal :type Vector))
  (bind _returnvalue (Transformation|GetActorForwardVector))
  (bind _returnvalue_2 (Math|Vector|GetReflectionVector _returnvalue SurfaceNormal))
  (if (!= HitMeteor self)
    (Physics|AddImpulse (Variables|Default|GetSM_Meteor) (* _returnvalue_2 1e+03) "None" false)
    (Variables|Default|SetCurrentDirection _returnvalue_2)))