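; Player character steered like a thrust-driven vehicle that can fire projectiles.
; MoveForward pushes the capsule along its forward vector with mass-independent force, limiting reverse to half strength; MoveRight feeds controller yaw and roll and clamps actor roll for banking.
; The Enhanced Input shoot action spawns BP_Projectile at the Cube component's transform, alongside legacy axis inputs.
; The Movement graph holds only unconnected movement and look-at nodes.
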(event Input|EnhancedActionEvents|EnhancedInputActionIA_Shoot
  (params (ActionValue :type Boolean) (ElapsedSeconds :type Float%20%28double-precision%29) (TriggeredSeconds :type Float%20%28double-precision%29) (InputAction :type Input%20Action%20Object%20Reference :default "/Game/Game/BP/Input/IA_Shoot.IA_Shoot"))
  (:Started
    (Game|SpawnActorfromClass "/Game/Game/BP/BP_Projectile.BP_Projectile_C" (Transformation|GetWorldTransform (Variables|Default|GetCube)) "Undefined" "MultiplyWithRoot" 0 0)))

(event EventBeginPlay)

(event Collision|EventActorBeginOverlap
  (params (OtherActor :type Actor%20Object%20Reference)))

(event EventTick
  (params (DeltaSeconds :type Float%20%28single-precision%29)))

(event Input|AxisEvents|InputAxisMoveForward
  (params (AxisValue :type Float%20%28single-precision%29))
  (Physics|AddForce (Variables|Collision|GetCapsuleComponent) (* (Math|Float|Clamp(Float) AxisValue -0.5) (Variables|Default|GetThrustSpeed) (Transformation|GetActorForwardVector)) "None" true))

(event Input|AxisEvents|InputAxisMoveRight
  (params (AxisValue :type Float%20%28single-precision%29))
  (bind _returnvalue (Transformation|GetActorRotation))
  (bind _returnvalue_2 (* AxisValue 0.7))
  (Pawn|Input|AddControllerYawInput _returnvalue_2)
  (Transformation|SetActorRotation (Math|Rotator|MakeRotator (Math|Float|Clamp(Float) (.roll _returnvalue) -3e+01 3e+01) (.pitch _returnvalue) (.yaw _returnvalue)))
  (Pawn|Input|AddControllerRollInput _returnvalue_2))

(event Input|EnhancedActionEvents|EnhancedInputActionIA_Movement
  (params (ActionValue :type Vector%202D%20Structure) (ElapsedSeconds :type Float%20%28double-precision%29) (TriggeredSeconds :type Float%20%28double-precision%29) (InputAction :type Input%20Action%20Object%20Reference :default "/Game/Game/BP/Input/IA_Movement.IA_Movement")))

(event EventLookat
  (params (Target :type Vector :default "0, 0, 0")))

(fn ConstructionScript)