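; BP_Projectile is a projectile that destroys meteors and awards score to the player.
; Overlaps on its Co_HitMeteor component call DestroyMeteors, which accepts only exact class matches for regular, missile and cluster meteors.
; A hit adds points to BP_Character's PlayerScore, removes the meteor from every BP_PlayerBounds PastCollided list, then destroys it.
; The projectile does not destroy itself in these graphs.
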(event OnComponentBeginOverlap(Co_HitMeteor)
  (params (OverlappedComponent :type Primitive%20Component%20Object%20Reference) (OtherActor :type Actor%20Object%20Reference) (OtherComp :type Primitive%20Component%20Object%20Reference) (OtherBodyIndex :type Integer) (bFromSweep :type Boolean) (SweepResult :type Hit%20Result%20Structure%20%28by%20ref%29))
  (CallFunction|DestroyMeteors OtherActor))

(event EventBeginPlay)

(event Collision|EventActorBeginOverlap
  (params (OtherActor :type Actor%20Object%20Reference)))

(event EventTick
  (params (DeltaSeconds :type Float%20%28single-precision%29)))

(fn ConstructionScript)

(fn DestroyMeteors
  (params (ActorCollided :type Actor%20Object%20Reference))
  (bind _returnvalue (Game|GetPlayerCharacter 0))
  (bind _returnvalue_2 (Utilities|GetClass ActorCollided))
  (bind _asbp_character (Utilities|Casting|CastToBP_Character _returnvalue))
  (if (Math|Boolean|ORBoolean (== _returnvalue_2 "/Game/Game/BP/BP_Meteor.BP_Meteor_C") (== _returnvalue_2 "/Game/Game/BP/BP_MissileMeteor.BP_MissileMeteor_C") (== _returnvalue_2 "/Game/Game/BP/BP_ClusterMeteor.BP_ClusterMeteor_C"))
    (Variables|/Game/Game/BP/BP_Character.BP_Character_C|SetPlayerScore _asbp_character (+ (Variables|/Game/Game/BP/BP_Character.BP_Character_C|GetPlayerScore _asbp_character) 10))
    (bind _outactors (Actor|GetAllActorsOfClass "/Game/Game/BP/BP_PlayerBounds.BP_PlayerBounds_C"))
    (for _array_element _outactors
      (if (Utilities|Map|Contains (Variables|/Game/Game/BP/BP_PlayerBounds.BP_PlayerBounds_C|GetPastCollided _array_element) ActorCollided)
        (Utilities|Map|Remove (Variables|/Game/Game/BP/BP_PlayerBounds.BP_PlayerBounds_C|GetPastCollided _array_element) ActorCollided)))
    (Actor|DestroyActor ActorCollided)))