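; Meteor hazard that alternates between aiming at the player and launching itself like a missile.
; When nearly stopped, it turns toward the player in fixed per-tick yaw steps, and a resettable DoOnce starts the timer for FireMissile.
; Firing applies a forward velocity-change impulse and holds the launch yaw until it slows again.
; Overlapping BP_Character deals damage, removes the meteor from BP_PlayerBounds' PastCollided lists and destroys it.
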(event OnComponentBeginOverlap(Co_MeteorHit)
  (params (OverlappedComponent :type Primitive%20Component%20Object%20Reference) (OtherActor :type Actor%20Object%20Reference) (OtherComp :type Primitive%20Component%20Object%20Reference) (OtherBodyIndex :type Integer) (bFromSweep :type Boolean) (SweepResult :type Hit%20Result%20Structure%20%28by%20ref%29))
  (bind _asbp_character (Utilities|Casting|CastToBP_Character OtherActor))
  (Game|Damage|ApplyDamage _asbp_character 1e+01 0 self)
  (bind _outactors (Actor|GetAllActorsOfClass "/Game/Game/BP/BP_PlayerBounds.BP_PlayerBounds_C"))
  (for _array_element _outactors
    (if (Utilities|Map|Contains (Variables|/Game/Game/BP/BP_PlayerBounds.BP_PlayerBounds_C|GetPastCollided _array_element) self)
      (Utilities|Map|Remove (Variables|/Game/Game/BP/BP_PlayerBounds.BP_PlayerBounds_C|GetPastCollided _array_element) self)))
  (Actor|DestroyActor))

(event EventBeginPlay)

(event EventTick
  (params (DeltaSeconds :type Float%20%28single-precision%29))
  (if (Variables|Default|GetIsTargeting)
    (CallFunction|LookatPlayer)
    (Utilities|FlowControl|DoOnce false :!label _label
      (:Completed
        (Utilities|Time|SetTimerbyFunctionName 0 "FireMissile" 3.0)
        (Utilities|FlowControl|Delay 1.0)))
    (elif (<= (Math|Vector|VectorLength (Transformation|GetVelocity)) 1e+01)
      (Variables|Default|SetIsTargeting true)
      (goto _label Reset)
      (else
        (Transformation|SetActorRotation (Math|Rotator|MakeRotator 0.0 0.0 (Variables|Default|GetPropulsionYaw)))))))

(fn ConstructionScript)

(fn FireMissile
  (Variables|Default|SetIsTargeting false)
  (Variables|Default|SetPropulsionYaw (.yaw (Transformation|GetActorRotation)))
  (Physics|AddImpulse (Variables|Default|GetSphere) (* (Transformation|GetActorForwardVector) 3e+03) "None" true))

(fn LookatPlayer
  (bind _returnvalue (Transformation|GetActorRotation))
  (bind _returnvalue_2 (Transformation|GetActorLocation))
  (bind _returnvalue_3 (Game|GetPlayerCharacter 0))
  (bind _returnvalue_4 (Transformation|GetActorLocation _returnvalue_3))
  (bind _returnvalue_5 (Math|Rotator|FindLookatRotation _returnvalue_2 _returnvalue_4))
  (if (> (.yaw _returnvalue_5) (.yaw _returnvalue))
    (Class|Actor|AddActorWorldRotation (Math|Rotator|MakeRotator 0.0 0.0 2.0))
    (elif (< (.yaw _returnvalue_5) (.yaw _returnvalue))
      (Class|Actor|AddActorWorldRotation (Math|Rotator|MakeRotator 0.0 0.0 -2.0)))))