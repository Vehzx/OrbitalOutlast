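; Player ship character that flies by capsule thrust with limited reverse, turns through controller input, and fires projectiles.
; Shooting spawns BP_Projectile at the capsule, with a looping timer repeating fire until input ends.
; Damage updates a health widget created on BeginPlay, and reaching zero opens a level.
; Q briefly slows global time, gated by a cooldown flag.
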(event Custom|Death
  (Game|OpenLevel(byObjectReference) "/Game/Level/Default.Default"))

(event Input|EnhancedActionEvents|EnhancedInputActionIA_Shoot
  (params (ActionValue :type Boolean) (ElapsedSeconds :type Float%20%28double-precision%29) (TriggeredSeconds :type Float%20%28double-precision%29) (InputAction :type Input%20Action%20Object%20Reference :default "/Game/Game/BP/Input/IA_Shoot.IA_Shoot"))
  (:Triggered
    (if (not (Utilities|Time|IsValidTimerHandle (Variables|Default|GetFiringTimer)))
      (bind _returnvalue (Utilities|Time|SetTimerbyFunctionName 0 "SpawnBullet" 0.1 true 1e-05))
      (Variables|Default|SetFiringTimer _returnvalue)))
  (:Started
    (CallFunction|SpawnBullet))
  (:Canceled
    (Utilities|Time|ClearandInvalidateTimerbyHandle (Variables|Default|GetFiringTimer) :!label _label))
  (:Completed
    (goto _label)))

(event EventBeginPlay
  (bind _returnvalue (UserInterface|CreateWidget "/Game/Game/UI/BP_health.BP_health_C"))
  (bind _output_get (Variables|Default|SethealthRef _returnvalue))
  (UserInterface|Viewport|AddtoViewport _output_get 0)
  (Variables|Default|SetCurrentHealth (Variables|Default|GetMaxHealth)))

(event Collision|EventActorBeginOverlap
  (params (OtherActor :type Actor%20Object%20Reference)))

(event Game|Damage|EventAnyDamage
  (params (Damage :type Float%20%28single-precision%29) (DamageType :type Damage%20Type%20Object%20Reference) (InstigatedBy :type Controller%20Object%20Reference) (DamageCauser :type Actor%20Object%20Reference))
  (bind _output_get (Variables|Default|SetCurrentHealth (Math|Float|Clamp(Float) (- (Variables|Default|GetCurrentHealth) Damage) 0.0 (Variables|Default|GetMaxHealth))))
  (Default|UpdateHealth (Variables|Default|GetHealthRef) _output_get (Variables|Default|GetMaxHealth))
  (if (<= _output_get 0.0)
    (CallFunction|Death)))

(event EventTick
  (params (DeltaSeconds :type Float%20%28single-precision%29)))

(event Input|AxisEvents|InputAxisMoveForward
  (params (AxisValue :type Float%20%28single-precision%29))
  ;[1 1 1] Forward Movement bacwards clamped to slow player
  (Physics|AddForce (Variables|Collision|GetCapsuleComponent) (* (Math|Float|Clamp(Float) AxisValue -0.5) (Variables|Default|GetThrustSpeed) (Transformation|GetActorForwardVector)) "None" true))

(event Input|AxisEvents|InputAxisMoveRight
  (params (AxisValue :type Float%20%28single-precision%29))
  (bind _returnvalue (Transformation|GetActorRotation))
  (bind _returnvalue_2 (* AxisValue 0.7))
  ;[1 1 1] Ship Rotation for firing has some logic for a roll effect not yet used as its hard to tell if it adds anything to the experience
  (Pawn|Input|AddControllerYawInput _returnvalue_2)
  (Transformation|SetActorRotation (Math|Rotator|MakeRotator (Math|Float|Clamp(Float) (+ (.roll _returnvalue) 1.0) -45.0 45.0) (.pitch _returnvalue) (.yaw _returnvalue)) true)
  (Pawn|Input|AddControllerRollInput _returnvalue_2))

(event Input|KeyboardEvents|Q
  (params (Key :type Key%20Structure :default "None"))
  ;[1 1 1] Slow time ability, 10 second cooldown (needs a visual timer on screen for cd) - luke
  (:Pressed
    (if (Variables|Default|GetQCooldown)
      (Utilities|FlowControl|Sequence
        (:then_0
          (Variables|Default|SetQCooldown false)
          (Utilities|Time|SetGlobalTimeDilation 0.2)
          (Utilities|FlowControl|Delay 1.0)
          (Utilities|Time|SetGlobalTimeDilation 1.0))
        (:then_1
          (Utilities|FlowControl|Delay 1e+01)
          (Variables|Default|SetQCooldown true))))))

(fn ConstructionScript)

(fn SpawnBullet
  (Game|SpawnActorfromClass "/Game/Game/BP/BP_Projectile.BP_Projectile_C" (Transformation|GetWorldTransform (Variables|Collision|GetCapsuleComponent)) "Undefined" "MultiplyWithRoot" 0 0))