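; Boundary portal that wraps the player character, meteors and projectiles around to a LinkedPortal.
; Overlap events track those actors with their entry locations, and Tick tests each for a front-to-back crossing of a plane through that point.
; Teleporting mirrors directions through both portals' transforms, also remapping control rotation and velocity once IsPlayer is set.
; Crossing history and IsPlayer are single variables shared by all tracked actors.
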(event OnComponentBeginOverlap(Co_PlayerBoundary)
  (params (OverlappedComponent :type Primitive%20Component%20Object%20Reference) (OtherActor :type Actor%20Object%20Reference) (OtherComp :type Primitive%20Component%20Object%20Reference) (OtherBodyIndex :type Integer) (bFromSweep :type Boolean) (SweepResult :type Hit%20Result%20Structure%20%28by%20ref%29))
  (bind (_castedactor _checksuccess) (CallFunction|IsGamePart OtherActor))
  (if _checksuccess
    (if (not (Utilities|Map|Contains (Variables|Default|GetCollidedActors) _castedactor))
      (Utilities|Map|Add (Variables|Default|GetCollidedActors) _castedactor (Transformation|GetActorLocation _castedactor))
      (Development|PrintString "Hello"))))

(event OnComponentEndOverlap(Co_PlayerBoundary)
  (params (OverlappedComponent :type Primitive%20Component%20Object%20Reference) (OtherActor :type Actor%20Object%20Reference) (OtherComp :type Primitive%20Component%20Object%20Reference) (OtherBodyIndex :type Integer))
  (Variables|Default|SetExitingActor OtherActor)
  (if (Utilities|Map|Contains (Variables|Default|GetCollidedActors) OtherActor)
    (Utilities|Map|Remove (Variables|Default|GetCollidedActors) (Variables|Default|GetExitingActor))))

(event EventBeginPlay)

(event Collision|EventActorBeginOverlap
  (params (OtherActor :type Actor%20Object%20Reference)))

(event EventTick
  (params (DeltaSeconds :type Float%20%28single-precision%29))
  (CallFunction|ShouldTeleport))

(fn ConstructionScript)

(fn ShouldTeleport
  (if (Utilities|Map|IsNotEmpty (Variables|Default|GetCollidedActors))
    (bind _keys (Utilities|Map|Keys (Variables|Default|GetCollidedActors)))
    (for _array_element _keys
      (bind _crossingportal (CallFunction|IsCrossingPortal (Transformation|GetActorLocation _array_element) (.Value (Utilities|Map|Find (Variables|Default|GetCollidedActors) _array_element)) (Math|Vector|GetForwardVector (Variables|Default|GetForwardDirection))))
      (if _crossingportal
        (CallFunction|TeleportActor _array_element)))))

(fn TeleportActor
  (params (CurrentActor :type Actor%20Object%20Reference))
  (bind _returnvalue (Game|GetPlayerCharacter 0))
  (bind _returnvalue_2 (Transformation|GetActorRotation))
  (bind _returnvalue_3 (Game|GetPlayerController 0))
  (bind _collidedactors (Variables|Default|GetCollidedActors))
  (bind _value (Utilities|Map|Find _collidedactors CurrentActor))
  (bind (_x _y _z) (Math|Rotator|BreakRotIntoAxes _returnvalue_2))
  (bind _returnvalue_4 (Pawn|GetControlRotation _returnvalue_3 :!class /Script/Engine.Controller))
  (bind _asbp_character (Utilities|Casting|CastToBP_Character _returnvalue))
  (bind _returnvalue_5 (Pawn|GetMovementComponent _asbp_character))
  (bind (_x_2 _y_2 _z_2) (Math|Rotator|BreakRotIntoAxes _returnvalue_4))
  (Transformation|SetActorTransform CurrentActor (Math|Transform|MakeTransform (CallFunction|UpdateLocation (Transformation|GetActorLocation) _value CurrentActor) (CallFunction|MirrorAxis (Utilities|Array|MakeArray _x _y _z) _value) (Transformation|GetActorScale3D CurrentActor)) false true)
  (if (Variables|Default|GetIsPlayer)
    (Pawn|SetControlRotation _returnvalue_3 (CallFunction|MirrorAxis (Utilities|Array|MakeArray _x_2 _y_2 _z_2) (.Value (Utilities|Map|Find (Variables|Default|GetCollidedActors) CurrentActor))))
    (Variables|/Script/Engine.MovementComponent|SetVelocity _returnvalue_5 (CallFunction|UpdateVelocity (Variables|/Script/Engine.MovementComponent|GetVelocity _returnvalue_5) (.Value (Utilities|Map|Find (Variables|Default|GetCollidedActors) CurrentActor)) _asbp_character))))

(fn IsCrossingPortal
  (params (CrossingPoint :type Vector) (WraparoundLocation :type Vector) (WraparoundNormal :type Vector))
  (LocalVariables|SetIsInFront (>= (Math|Vector|DotProduct (- CrossingPoint WraparoundLocation) WraparoundNormal) 0.0))
  (bind _output_get (LocalVariables|SetWrapAroundPlane (Class|KismetMathLibrary|MakePlanefromPointandNormal WraparoundLocation WraparoundNormal)))
  (bind _output_get_2 (LocalVariables|SetIsIntersecting (.ReturnValue (Class|KismetMathLibrary|LinePlaneIntersection (Variables|Default|GetLastPosition) CrossingPoint _output_get))))
  (LocalVariables|SetIsCrossing (Math|Boolean|ANDBoolean _output_get_2 (not (LocalVariables|GetIsInFront)) (Variables|Default|GetLastInFront)))
  (Variables|Default|SetLastInFront (LocalVariables|GetIsInFront))
  (Variables|Default|SetLastPosition CrossingPoint)
  (return (LocalVariables|GetIsCrossing)))

(fn IsGamePart
  (params (OverlappedActor :type Actor%20Object%20Reference))
  (bind _asbp_character (Utilities|Casting|CastToBP_Character OverlappedActor)
    (:then
      (Variables|Default|SetIsPlayer true)
      (return _asbp_character true))
    (:CastFailed
      (bind _asbp_meteor (Utilities|Casting|CastToBP_Meteor OverlappedActor)
        (:then
          (return _asbp_meteor true))
        (:CastFailed
          (bind _asbp_projectile (Utilities|Casting|CastToBP_Projectile OverlappedActor)
            (:then
              (return _asbp_projectile true))
            (:CastFailed
              (return 0 false))))))))

(fn MirrorAxis
  (params (OldAxes :type Array%20of%20Vectors) (CollisionPoint :type Vector))
  (for _index (range 0 (- (Utilities|Array|Length OldAxes) 1))
    (Utilities|Array|SetArrayElem OldAxes _index (CallFunction|SwitchDirection (Utilities|Array|Get(acopy) OldAxes _index) CollisionPoint)))
  (return (Math|Rotator|MakeRotationfromAxes (Utilities|Array|Get(acopy) OldAxes) (Utilities|Array|Get(acopy) OldAxes 1) (Utilities|Array|Get(acopy) OldAxes 2))))

(fn SwitchDirection
  (params (InitialDirection :type Vector) (CollisionPoint :type Vector))
  (return (Math|Transform|TransformDirection (Transformation|GetActorTransform (Variables|Default|GetLinkedPortal)) (Math|Vector|MirrorVectorbyNormal (Math|Vector|MirrorVectorbyNormal (Math|Transform|InverseTransformDirection (Transformation|GetActorTransform) InitialDirection) "1.000000,0.000000,0.000000") "0.000000,1.000000,0.000000"))))

(fn UpdateLocation
  (params (OldLocation :type Vector) (CollisionPoint :type Vector) (Actor :type Actor%20Object%20Reference))
  (bind _returnvalue (Transformation|GetActorTransform Actor))
  (return (+ (* (* (Math|Vector|GetUnitDirection(Vector) OldLocation CollisionPoint) 1.0) (Math|Vector|Distance(Vector) OldLocation CollisionPoint)) (Math|Transform|TransformLocation (Transformation|GetActorTransform (Variables|Default|GetLinkedPortal)) (Math|Transform|InverseTransformLocation (Math|Transform|MakeTransform (LocalVariables|GetCollisionpoint) (.rotation _returnvalue) (Math|Vector|MakeVector (* (.x (.scale _returnvalue)) -1.0) (* (.y (.scale _returnvalue)) -1.0) (.z (.scale _returnvalue)))) CollisionPoint)))))

(fn UpdateVelocity
  (params (OldVelocity :type Vector) (CollisionPoint :type Vector) (AppliedActor :type BP%20Character%20Object%20Reference))
  (return (* (CallFunction|SwitchDirection (Math|Vector|Normalize OldVelocity) CollisionPoint) (Math|Vector|VectorLength (Transformation|GetVelocity AppliedActor)))))